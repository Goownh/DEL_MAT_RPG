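; BP_ItemInGame is a world pickup that represents the item held in its CurrentItem data.
; On BeginPlay it applies that item's mesh, icon sprite and name to its mesh, sprite and text components.
; Tick turns the mesh and name text to face the player camera.
; When the top-down character overlaps its sphere, it passes the item to the player controller's AddItem and destroys itself.
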(event OnComponentBeginOverlap(Sphere)
  (params (OverlappedComponent :type Primitive%20Component%20Object%20Reference) (OtherActor :type Actor%20Object%20Reference) (OtherComp :type Primitive%20Component%20Object%20Reference) (OtherBodyIndex :type Integer) (bFromSweep :type Boolean) (SweepResult :type Hit%20Result%20Structure%20%28by%20ref%29))
  ;[0.15 0.15 0.15 0.5] Add Item to Inv
  (Utilities|Casting|CastToBP_TopDownCharacter OtherActor)
  (Default|AddItem (CallFunction|GetTopDownController) (Variables|Default|GetCurrentItem))
  (Actor|DestroyActor))

(event EventBeginPlay
  (bind _currentitem (Variables|Default|GetCurrentItem))
  ;[0.15 0.15 0.15 0.5] Set Item Mesh and Name
  (Components|StaticMesh|SetStaticMesh (Variables|Default|GetStaticMesh) (Variables|/Game/Blueprint/Data/BP_DA_Item.BP_DA_Item_C|GetMesh _currentitem))
  (Rendering|Components|Sprite|SetSprite (Variables|Default|GetPaperSprite) (Variables|/Game/Blueprint/Data/BP_DA_Item.BP_DA_Item_C|GetIcone _currentitem))
  (Rendering|Components|TextRender|SetText (Variables|Default|GetTextRender) (Variables|/Game/Blueprint/Data/BP_DA_Item.BP_DA_Item_C|GetName _currentitem)))

(event EventTick
  (params (DeltaSeconds :type Float%20%28single-precision%29))
  (bind _asbp_top_down_controller (CallFunction|GetTopDownController))
  (bind _textrender (Variables|Default|GetTextRender))
  (bind _staticmesh (Variables|Default|GetStaticMesh))
  (bind _playercameramanager (Variables|/Script/Engine.PlayerController|GetPlayerCameraManager _asbp_top_down_controller))
  (bind _returnvalue (Camera|GetCameraLocation _playercameramanager))
  ;[0.15 0.15 0.15 0.5] Make Mesh+Name Rotate to Camera Player
  (Transformation|SetWorldRotation _textrender (Math|Rotator|FindLookatRotation (Transformation|GetWorldLocation _textrender) _returnvalue) false false)
  (Transformation|SetWorldRotation _staticmesh (Math|Rotator|FindLookatRotation (Transformation|GetWorldLocation _staticmesh) _returnvalue) false false))

(fn ConstructionScript)