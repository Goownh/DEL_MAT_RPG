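; BP_ItemInGame is an interactable world pickup that displays an item's icon and name.
; On BeginPlay it fills a PaperSprite and TextRender from its CurrentItem data.
; Each Tick it rotates the name text to face the top-down camera.
; A sphere overlap casts for BP_TopDownCharacter but triggers no further action yet.
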(event OnComponentBeginOverlap(Sphere)
  (params (OverlappedComponent :type Primitive%20Component%20Object%20Reference) (OtherActor :type Actor%20Object%20Reference) (OtherComp :type Primitive%20Component%20Object%20Reference) (OtherBodyIndex :type Integer) (bFromSweep :type Boolean) (SweepResult :type Hit%20Result%20Structure%20%28by%20ref%29))
  (Utilities|Casting|CastToBP_TopDownCharacter OtherActor))

(event EventBeginPlay
  (bind _currentitem (Variables|Default|GetCurrentItem))
  (Rendering|Components|Sprite|SetSprite (Variables|Default|GetPaperSprite) (Variables|/Game/Blueprint/Data/BP_DA_Item.BP_DA_Item_C|GetIcone _currentitem))
  (Rendering|Components|TextRender|SetText (Variables|Default|GetTextRender) (Variables|/Game/Blueprint/Data/BP_DA_Item.BP_DA_Item_C|GetName _currentitem)))

(event EventTick
  (params (DeltaSeconds :type Float%20%28single-precision%29))
  (bind _textrender (Variables|Default|GetTextRender))
  (Transformation|SetWorldRotation _textrender (Math|Rotator|FindLookatRotation (Transformation|GetWorldLocation _textrender) (Camera|GetCameraLocation (Variables|/Script/Engine.PlayerController|GetPlayerCameraManager (CallFunction|GetTopDownController)))) false false))

(fn ConstructionScript)