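; BP_PNJ is an interactable NPC that toggles a talk state each time its Interact event fires.
; A FlipFlop first shows its text render, blends the view to the NPC, disables player movement and sets the top-down controller's Talk flag.
; The next interaction hides the text, blends the view back to the controlled pawn, restores walking and clears Talk.
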(event EventInterract
  (bind _asbp_top_down_controller (CallFunction|GetTopDownController))
  (bind _asbp_top_down_controller_2 (CallFunction|GetTopDownController))
  (bind _textrender1 (Variables|Default|GetTextRender1))
  (Utilities|FlowControl|FlipFlop
    (:A
      (Rendering|SetVisibility _textrender1 true false)
      (Game|Player|SetViewTargetwithBlend (CallFunction|GetTopDownController) self 0.5 "VTBlend_Linear" 0.0 false)
      (Pawn|Components|CharacterMovement|SetMovementMode (Variables|/Script/Engine.Character|GetCharacterMovement (Game|GetPlayerCharacter 0)) "MOVE_None" 0)
      (Variables|/Game/Blueprint/TopDownCharacter/BP_TopDownController.BP_TopDownController_C|SetTalk _asbp_top_down_controller true))
    (:B
      (Rendering|SetVisibility _textrender1 false false)
      (Game|Player|SetViewTargetwithBlend _asbp_top_down_controller_2 (Pawn|GetControlledPawn _asbp_top_down_controller_2) 0.5 "VTBlend_Linear" 0.0 false)
      (Pawn|Components|CharacterMovement|SetMovementMode (Variables|/Script/Engine.Character|GetCharacterMovement (Game|GetPlayerCharacter 0)) "MOVE_Walking" 0)
      (Variables|/Game/Blueprint/TopDownCharacter/BP_TopDownController.BP_TopDownController_C|SetTalk _asbp_top_down_controller false))))

(fn ConstructionScript
  (|CallParentFunction))